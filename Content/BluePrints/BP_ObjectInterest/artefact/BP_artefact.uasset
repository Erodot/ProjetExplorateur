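; BP_artefact is an object-of-interest actor that reveals its WidgetDisplay when something overlaps its DetectionBox.
; On BeginPlay it disables the widget's collision.
; Overlap begin shows the widget and enables query-only collision, while overlap end hides it and disables collision again, each printing a debug string.
; The overlap events do not filter which actor triggers them.
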(event OnComponentBeginOverlap(DetectionBox)
  (params (OverlappedComponent :type Primitive%20Component%20Object%20Reference) (OtherActor :type Actor%20Object%20Reference) (OtherComp :type Primitive%20Component%20Object%20Reference) (OtherBodyIndex :type Integer) (bFromSweep :type Boolean) (SweepResult :type Hit%20Result%20Structure%20%28by%20ref%29))
  (bind _widgetdisplay (Variables|Default|GetWidgetDisplay))
  (Development|PrintString "In")
  (Rendering|SetVisibility _widgetdisplay true false)
  (Collision|SetCollisionEnabled _widgetdisplay "QueryOnly"))

(event OnComponentEndOverlap(DetectionBox)
  (params (OverlappedComponent :type Primitive%20Component%20Object%20Reference) (OtherActor :type Actor%20Object%20Reference) (OtherComp :type Primitive%20Component%20Object%20Reference) (OtherBodyIndex :type Integer))
  (bind _widgetdisplay (Variables|Default|GetWidgetDisplay))
  (Development|PrintString "Out")
  (Rendering|SetVisibility _widgetdisplay false false)
  (Collision|SetCollisionEnabled _widgetdisplay "NoCollision"))

(event Collision|EventActorBeginOverlap
  (params (OtherActor :type Actor%20Object%20Reference)))

(event EventTick
  (params (DeltaSeconds :type Float%20%28single-precision%29)))

(event EventBeginPlay
  (Collision|SetCollisionEnabled (Variables|Default|GetWidgetDisplay) "NoCollision"))

(fn ConstructionScript)