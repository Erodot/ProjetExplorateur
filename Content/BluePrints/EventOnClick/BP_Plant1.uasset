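; BP_Plant1 is a clickable plant actor that toggles a UI pop-up.
; On BeginPlay it creates a BP_UIClickable widget and adds it to the viewport.
; Clicks and touches on the interactable sprite share one FlipFlop that alternately shows and hides that widget.
; An unconnected older branch toggles a pop-up flag on WBP_InGameUI instead and never runs.
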(event OnClicked(Sprite_Interactable)
  (params (TouchedComponent :type Primitive%20Component%20Object%20Reference) (ButtonPressed :type Key%20Structure :default "None"))
  (bind _widgetpopup (Variables|Default|GetWidgetPopUp))
  (Utilities|FlowControl|FlipFlop
    (:A
      (Widget|SetVisibility _widgetpopup "Visible"))
    (:B
      (Widget|SetVisibility _widgetpopup "Hidden"))))

(event OnInputTouchBegin(Sprite_Interactable)
  (params (FingerIndex :type ETouchIndex%20Enum :default "Touch1") (TouchedComponent :type Primitive%20Component%20Object%20Reference))
  (bind _widgetpopup (Variables|Default|GetWidgetPopUp))
  (Utilities|FlowControl|FlipFlop
    (:A
      (Widget|SetVisibility _widgetpopup "Visible"))
    (:B
      (Widget|SetVisibility _widgetpopup "Hidden"))))

(event EventBeginPlay
  (bind _returnvalue (UserInterface|CreateWidget "/Game/BluePrints/EventOnClick/BP_UIClickable.BP_UIClickable_C"))
  (bind _output_get (Variables|Default|SetWidgetPopUp _returnvalue))
  (UserInterface|Viewport|AddtoViewport _output_get 0))

(event Collision|EventActorBeginOverlap
  (params (OtherActor :type Actor%20Object%20Reference)))

(event EventTick
  (params (DeltaSeconds :type Float%20%28single-precision%29)))

(fn ConstructionScript)